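; BP_PlayerCam is a follow camera that tracks a chosen actor from a fixed offset.
; On BeginPlay it makes itself the view target of player 0's BP_customController.
; Each Tick it smoothly interpolates toward the focus actor's location plus an offset, pulled back along negative Y by a set distance.
; The target also adds the actor's scaled velocity, so the camera leads the direction of movement.
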(event `self.ReceiveBeginPlay`
  (bind _asbp_custom_controller (cast `/Game/blueprints/core/BP_customController` (`GameplayStatics.GetPlayerController` 0)))
  (`PlayerController.SetViewTargetWithBlend` _asbp_custom_controller self 0.0 "VTBlend_Linear" 0.0 true))

(event `self.ReceiveTick`
  (params (DeltaSeconds :type "Float (single-precision)"))
  (bind _focuswhichactor (`self.focusWhichActor`))
  (`self.K2_SetActorLocation` (`KismetMathLibrary.VInterpTo` (`self.K2_GetActorLocation`) (+ (+ (+ (`self.K2_GetActorLocation` _focuswhichactor) (`self.offSetCam`)) (`KismetMathLibrary.MakeVector` 0.0 (* (`self.distanceFromActor`) -1.0))) (* (`self.GetVelocity` _focuswhichactor) (`self.distanceInfrontOfPlayer`))) DeltaSeconds (`self.Interp Speed`))))

(fn `UserConstructionScript`)