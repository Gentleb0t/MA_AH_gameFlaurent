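; Actor component that lets its owning pawn hack other actors, hopping control between pawns and back.
; It sphere-traces from the owner toward the mouse cursor, projected onto the owner's Y-normal plane, and accepts hit actors implementing BPI_Interact.
; Hacking unpossesses the controller and messages the target with the controller, previous pawn, decremented jump count and camera.
; Return functions hand control to the last pawn or the game mode's origin pawn.
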(event `self.ReceiveBeginPlay`
  (bind _asbp_in_game_controller (cast `/Game/blueprints/core/BP_InGameController` (`GameplayStatics.GetPlayerController` 0)))
  (set `self.As Controller` _asbp_in_game_controller))

(fn `hackObject`
  (params (ActorToHack :type "Pawn Object Reference") (nbremainingJUmp :type Integer))
  (if true
    (`|ExecutionSequence`
      (:`then_0`
        (`Controller.UnPossess` (`self.As Controller`))
        (set `self.PawnInputs` "NewEnumerator0"))
      (:`then_1`
        (message `/Game/blueprints/core/BPI_Interact.HackObject` ActorToHack (`self.As Controller`) (cast `Pawn` (`self.GetOwner`) :!pure true) (- nbremainingJUmp 1) (`self.RefCam`))
        (set `self.PawnInputs` "NewEnumerator0")))))

(fn `HackTerminal`
  (params (actor :type "Actor Object Reference"))
  (message `/Game/blueprints/core/BPI_Interact.interactWithObject` actor))

(fn `returnToLastActorPosses`
  (params (LastActor :type "Pawn Object Reference"))
  (bind _as_controller (`self.As Controller`))
  (`Controller.UnPossess` _as_controller)
  (message `/Game/blueprints/core/BPI_Interact.returnToLastActorPosses` LastActor _as_controller)
  (set `self.PawnInputs` "NewEnumerator0"))

(fn `returnToPawnPlayer`
  (`Controller.UnPossess` (`self.As Controller`))
  (message `/Game/blueprints/core/BPI_Interact.returnToPawnPlayer` (`/Game/blueprints/core/BP_customGameMode.OriginPawn` (cast `/Game/blueprints/core/BP_customGameMode` (`GameplayStatics.GetGameMode`) :!pure true)) (`self.As Controller`))
  (set `self.PawnInputs` "NewEnumerator0"))

(fn `setObjectToHack`
  (returns (`Hit Result Hit Actor` :type "Actor Object Reference"))
  (bind (_hit_result_bblockinghit _hit_result_binitialoverlap _hit_result_time _hit_result_distance _hit_result_location _hit_result_impactpoint _hit_result_normal _hit_result_impactnormal _hit_result_physmat _hit_result_hitactor) (`GameplayStatics.BreakHitResult` (`self.TraceHack`)))
  (if (`KismetSystemLibrary.DoesImplementInterface` _hit_result_hitactor "/Game/blueprints/core/BPI_Interact.BPI_Interact_C")
    (return _hit_result_hitactor)
    (else
      (return null))))

(fn `TraceHack`
  (returns (`hit result` :type "HitResult Structure"))
  (bind (_worldlocation _worlddirection) (`PlayerController.DeprojectMousePositionToWorld` (`self.as Controller`)))
  (if (`|EnumEquality` (`self.PawnInputs`) "NewEnumerator3")
    (`KismetSystemLibrary.PrintString` "Hello")
    (bind _outhit (`KismetSystemLibrary.SphereTraceSingle` :`Start` (`Actor.K2_GetActorLocation` (`self.GetOwner`)) :`End` (`.Intersection` (`KismetMathLibrary.LinePlaneIntersection_OriginNormal` _worldlocation (* _worlddirection 1000000.0) (`Actor.K2_GetActorLocation` (`self.GetOwner`)) (0.0 1.0 0.0))) :`Radius` 5.0 :`TraceChannel` "TraceTypeQuery1" :`DrawDebugType` "ForOneFrame"))
    (return _outhit)))