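; Player controller that manages Enhanced Input mapping contexts for normal and hacking play.
; BeginPlay adds the character and hack contexts at the same priority.
; SwitchInputs adds by mode, though Normal sets no context and Hacking adds IMC_Character.
; RemoveMappingContext removes the character context for Normal and the hacked drone context for Hacking, which this controller never adds.
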(event `self.ReceiveBeginPlay`
  (`|ExecutionSequence`
    (:`then_0`
      (`EnhancedInputSubsystemInterface.AddMappingContext` (subsystem `EnhancedInputLocalPlayerSubsystem`) "/Game/blueprints/core/Inputs/IMC_Character.IMC_Character" 0 (struct)))
    (:`then_1`
      (`EnhancedInputSubsystemInterface.AddMappingContext` (subsystem `EnhancedInputLocalPlayerSubsystem`) "/Game/blueprints/core/Inputs/IMC_Hack.IMC_Hack" 0 (struct)))))

(fn `removeMappingContext`
  (params (WhatToRemove :type "/Game/blueprints/core/E_PlayerState Enum" :default "NewEnumerator0"))
  (switch `/Game/blueprints/core/E_PlayerState` WhatToRemove
    (:`NewEnumerator0`
      (`EnhancedInputSubsystemInterface.RemoveMappingContext` (subsystem `EnhancedInputLocalPlayerSubsystem`) "/Game/blueprints/core/Inputs/IMC_Character.IMC_Character" (struct)))
    (:`NewEnumerator3`
      (`EnhancedInputSubsystemInterface.RemoveMappingContext` (subsystem `EnhancedInputLocalPlayerSubsystem`) "/Game/blueprints/core/Inputs/IMC_HackedDrone.IMC_HackedDrone" (struct)))))

(fn `switchInputs`
  (params (WhatsNewInputs :type "/Game/blueprints/core/E_PlayerState Enum" :default "NewEnumerator0"))
  (switch `/Game/blueprints/core/E_PlayerState` WhatsNewInputs
    (:`NewEnumerator0`
      (`EnhancedInputSubsystemInterface.AddMappingContext` (subsystem `EnhancedInputLocalPlayerSubsystem`) null 0 (struct)))
    (:`NewEnumerator3`
      (`EnhancedInputSubsystemInterface.AddMappingContext` (subsystem `EnhancedInputLocalPlayerSubsystem`) "/Game/blueprints/core/Inputs/IMC_Character.IMC_Character" 0 (struct)))))

(fn `UserConstructionScript`)