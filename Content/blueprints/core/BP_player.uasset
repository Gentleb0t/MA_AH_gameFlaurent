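; Player pawn that moves along its capsule's forward axis and can switch into a hacking mode to hack other pawns.
; It spawns a BP_PlayerCam shared with BPHackingComponent, which holds the input state, picks the target each tick and runs the hack.
; Return events refocus the camera and repossess the player.
; Being spotted disables input behind a black-fade widget, and a debug key clears playerRef on all AI blackboards.
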(event `self.ReceiveBeginPlay`
  (bind _returnvalue (`|SpawnActorFromClass` "/Game/blueprints/core/BP_PlayerCam.BP_PlayerCam_C" (`self.GetTransform`) "Undefined" "MultiplyWithRoot" null self (`self.offSetCamera`) null))
  (bind _output_get (set `self.CameraRef` _returnvalue))
  (set `/Game/blueprints/core/BP_hackingComponent.RefCam` _output_get (`self.BP_hackingComponent`))
  (bind _asbp_in_game_controller (cast `/Game/blueprints/core/BP_InGameController` (`GameplayStatics.GetPlayerController` 0)))
  (set `self.Controllers` _asbp_in_game_controller))

(event `EnhancedInput|/Game/blueprints/core/Inputs/InputsActions/IA_move`
  (params (ActionValue :type "Float (double-precision)") (ElapsedSeconds :type "Float (double-precision)") (TriggeredSeconds :type "Float (double-precision)") (InputAction :type "InputAction Object Reference" :default "/Game/blueprints/core/Inputs/InputsActions/IA_move.IA_move"))
  (:`Triggered`
    (if (`|EnumEquality` (`/Game/blueprints/core/BP_hackingComponent.PawnInputs` (`self.BP_hackingComponent`)) "NewEnumerator0")
      (`self.horizontalMovement` ActionValue))))

(event `EnhancedInput|/Game/blueprints/core/Inputs/InputsActions/IA_switchMode`
  (params (ActionValue :type Boolean) (ElapsedSeconds :type "Float (double-precision)") (TriggeredSeconds :type "Float (double-precision)") (InputAction :type "InputAction Object Reference" :default "/Game/blueprints/core/Inputs/InputsActions/IA_switchMode.IA_switchMode"))
  (:`Started`
    (set `/Game/blueprints/core/BP_hackingComponent.PawnInputs` (select `/Game/blueprints/core/E_PlayerState` (`/Game/blueprints/core/BP_hackingComponent.PawnInputs` (`self.BP_hackingComponent`)) :`NewEnumerator0` (enumliteral `/Game/blueprints/core/E_PlayerState` "NewEnumerator3") :`NewEnumerator3` "NewEnumerator0") (`self.BP_hackingComponent`))))

(event `EnhancedInput|/Game/blueprints/core/Inputs/InputsActions/IA_Hack`
  (params (ActionValue :type Boolean) (ElapsedSeconds :type "Float (double-precision)") (TriggeredSeconds :type "Float (double-precision)") (InputAction :type "InputAction Object Reference" :default "/Game/blueprints/core/Inputs/InputsActions/IA_Hack.IA_Hack"))
  (:`Started`
    (bind _whichobjecttohack (`self.WhichObjectToHack`)
      (:`then`
        (`/Game/blueprints/core/BP_hackingComponent.hackObject` (`self.BP_hackingComponent`) (cast `Pawn` _whichobjecttohack :!pure true) (`self.nbMaxDistanceHack`)))
      (:`else`))))

(event `self.ReceiveTick`
  (params (DeltaSeconds :type "Float (single-precision)"))
  (bind _hit_result_hit_actor (`/Game/blueprints/core/BP_hackingComponent.setObjectToHack` (`self.BP_hackingComponent`)))
  (set `self.WhichObjectToHack` _hit_result_hit_actor))

(event `/Game/blueprints/core/BPI_Interact.returnToLastActorPosses`
  (params (Controller :type "/Game/blueprints/core/BP_InGameController Object Reference"))
  (bind _refcam (`/Game/blueprints/core/BP_hackingComponent.RefCam` (`self.BP_hackingComponent`)))
  (set `/Game/blueprints/core/BP_PlayerCam.focusWhichActor` self _refcam)
  (set `/Game/blueprints/core/BP_PlayerCam.offSetCam` (`self.offSetCamera`) _refcam)
  (`Controller.Possess` Controller self))

(event `/Game/blueprints/core/BPI_Interact.returnToPawnPlayer`
  (params (Controller :type "/Game/blueprints/core/BP_InGameController Object Reference"))
  (bind _refcam (`/Game/blueprints/core/BP_hackingComponent.RefCam` (`self.BP_hackingComponent`)))
  (set `/Game/blueprints/core/BP_PlayerCam.focusWhichActor` self _refcam)
  (set `/Game/blueprints/core/BP_PlayerCam.offSetCam` (`self.offSetCamera`) _refcam)
  (`Controller.Possess` Controller self))

(event `Key|R`
  (params (Key :type "Key Structure"))
  ; debug
  (:`Pressed`
    (bind _outactors (`GameplayStatics.GetAllActorsOfClass` "/Game/blueprints/AI/BP_AI.BP_AI_C"))
    (for _array_element _outactors
      (`BlackboardComponent.ClearValue` (`AIBlueprintHelperLibrary.GetBlackboard` _array_element) "playerRef"))))

(event `/Game/blueprints/core/BPI_Common.isSpotted`
  (bind _returnvalue (`|CreateWidget` "/Game/blueprints/widgets/transition/WG_blackFade.WG_blackFade_C"))
  (`UserWidget.AddToViewport` _returnvalue 0)
  (set `self.refWidgetTransition` _returnvalue)
  (add `/Game/blueprints/widgets/transition/WG_blackFade.endFade` _returnvalue (`|CreateDelegate` :!event `RespawnPlayer`))
  (`self.DisableInput` (`self.Controllers`)))

(fn `functionDie`
  (`KismetSystemLibrary.PrintString` "mort"))

(fn `horizontalMovement`
  (params (direction :type "Float (double-precision)"))
  (`self.AddMovementInput` (`SceneComponent.GetForwardVector` (`self.CapsuleComponent`)) direction))

(fn `RespawnPlayer`
  (`/Game/blueprints/widgets/transition/WG_blackFade.fadeOut` (`self.refWidgetTransition`)))

(fn `UserConstructionScript`)