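; BP_elevator is an elevator actor that moves between its starting position and a relative offset when its receiver component is hacked.
; On begin play it stores its origin, binds the receiver's hacked event to the elevator toggle, and sets the timeline play rate from the trajectory time.
; Each hack alternates, via FlipFlop, between playing and reversing the timeline that lerps the actor's location.
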(event `self.ReceiveBeginPlay`
  (`parent.ReceiveBeginPlay`)
  (set `self.OrigineLocation` (`self.K2_GetActorLocation`))
  (add `/Game/blueprints/BP_Interactions.hacked` (`self.BP_receiver`) (delegate `playElevator`))
  (`TimelineComponent.SetPlayRate` (`self.elevator`) (/ 1.0 (`self.elevatorTrajectoryTime`))))

(event `playElevator`
  (`/Engine/EditorBlueprintResources/StandardMacros.FlipFlop`
    (:`A`
      (bind (_direction _newtrack_0) (`Timeline|elevator` :!label _label)
        (:`Update`
          (`self.K2_SetActorLocation` (`KismetMathLibrary.VLerp` (`self.OrigineLocation`) (+ (`self.DesiredLocation`) (`self.OrigineLocation`)) _newtrack_0)))))
    (:`B`
      (goto _label :!via `Reverse`))))

(fn `UserConstructionScript`
  (`parent.UserConstructionScript`))