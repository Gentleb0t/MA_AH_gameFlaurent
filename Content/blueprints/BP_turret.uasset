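; Hackable turret pawn that the player possesses, with the shared camera refocused on it, to aim and shoot with the mouse.
; Tick intersects the cursor ray with the turret's XZ plane and snaps the pivot's pitch to that point; the Speed-scaled pitch is never applied.
; Shoot input runs a looping timer, and Shoot line-traces from the arrow to send ShootedMessage.
; Releasing back returns control to the last possessed actor, or the player after a one-second hold.
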(event `self.ReceiveTick`
  (params (DeltaSeconds :type "Float (single-precision)"))
  (bind (_worldlocation _worlddirection) (`PlayerController.DeprojectMousePositionToWorld` (`self.Controller_0`)))
  (`parent.ReceiveTick` DeltaSeconds)
  (if (`self.isPossess`)
    (bind _output_get (set `self.targetPitch` (`KismetMathLibrary.DegAtan2` (.z (- (`.Intersection` (`KismetMathLibrary.LinePlaneIntersection_OriginNormal` _worldlocation (* _worlddirection 1000000.0) (`self.K2_GetActorLocation`) (0.0 1.0 0.0))) (`SceneComponent.K2_GetComponentLocation` (`self.rotationPoint`)))) (.x (- (`.Intersection` (`KismetMathLibrary.LinePlaneIntersection_OriginNormal` _worldlocation (* _worlddirection 1000000.0) (`self.K2_GetActorLocation`) (0.0 1.0 0.0))) (`SceneComponent.K2_GetComponentLocation` (`self.rotationPoint`)))))))
    (bind _returnvalue (`KismetMathLibrary.NormalizeAxis` (- _output_get (`self.currentPitch`))))
    (set `self.Delta` _returnvalue)
    (set `self.currentPitch` (* DeltaSeconds _returnvalue (`self.speed`)))
    (`SceneComponent.K2_SetWorldRotation` (`self.rotationPoint`) (`KismetMathLibrary.MakeRotator` 0.0 (`self.targetPitch`)) false false)))

(event `EnhancedInput|/Game/blueprints/core/Inputs/InputsActions/IA_shoot`
  (params (ActionValue :type Boolean) (ElapsedSeconds :type "Float (double-precision)") (TriggeredSeconds :type "Float (double-precision)") (InputAction :type "InputAction Object Reference" :default "/Game/blueprints/core/Inputs/InputsActions/IA_shoot.IA_shoot"))
  (:`Started`
    (if (`|EnumEquality` (`/Game/blueprints/core/BP_hackingComponent.PawnInputs` (`self.BP_hackingComponent`)) "NewEnumerator0")
      (`/Engine/EditorBlueprintResources/StandardMacros.DoOnce` false :!label _label
        (:`Completed`
          (bind _returnvalue (`KismetSystemLibrary.K2_SetTimerDelegate` (`|CreateDelegate` :!event `shoot`) (`self.ShootingRate`) true))
          (set `self.timerByEventShoot` _returnvalue)))))
  (:`Completed`
    (`KismetSystemLibrary.K2_ClearAndInvalidateTimerHandle` (`self.timerByEventShoot`))
    (goto _label :!via `Reset`)))

(event `/Game/blueprints/core/BPI_Interact.HackObject`
  (params (Controller :type "/Game/blueprints/core/BP_InGameController Object Reference") (lastActorPosses :type "Pawn Object Reference") (camRef :type "/Game/blueprints/core/BP_PlayerCam Object Reference"))
  (set `self.Controller_0` Controller)
  (set `self.lastActorPosses` lastActorPosses)
  (bind _output_get (set `/Game/blueprints/core/BP_hackingComponent.RefCam` camRef (`self.BP_hackingComponent`)))
  (set `/Game/blueprints/core/BP_PlayerCam.focusWhichActor` self _output_get)
  (set `/Game/blueprints/core/BP_PlayerCam.offSetCam` (`self.offsetCamera`) _output_get)
  (`Controller.Possess` (`self.Controller_0`) self)
  (set `self.isPossess` true))

(event `EnhancedInput|/Game/blueprints/core/Inputs/InputsActions/IA_backToLast`
  (params (ActionValue :type Boolean) (ElapsedSeconds :type "Float (double-precision)") (TriggeredSeconds :type "Float (double-precision)") (InputAction :type "InputAction Object Reference" :default "/Game/blueprints/core/Inputs/InputsActions/IA_backToLast.IA_backToLast"))
  (:`Triggered`
    (set `self.HoldToGetBackToPLayer` TriggeredSeconds))
  (:`Completed`
    (set `self.isPossess` false)
    (if (> (`self.HoldToGetBackToPLayer`) 1.0)
      (`/Game/blueprints/core/BP_hackingComponent.returnToPawnPlayer` (`self.BP_hackingComponent`))
      (else
        (`/Game/blueprints/core/BP_hackingComponent.returnToLastActorPosses` (`self.BP_hackingComponent`) (`self.lastActorPosses`))))))

(fn `shoot`
  (bind _arrow (`self.Arrow`))
  (bind _returnvalue (`SceneComponent.K2_GetComponentLocation` _arrow))
  (bind _outhit (`KismetSystemLibrary.LineTraceSingle` :`Start` _returnvalue :`End` (+ _returnvalue (* (`SceneComponent.GetForwardVector` _arrow) (`self.range`))) :`TraceChannel` "TraceTypeQuery1" :`DrawDebugType` "Persistent"))
  (message `/Game/blueprints/core/BPI_Common.shooted` (`.HitActor` (`GameplayStatics.BreakHitResult` _outhit))))

(fn `UserConstructionScript`
  (`parent.UserConstructionScript`))