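; Base pawn for hackable actors such as turrets, which the player's controller possesses by hacking, chaining from one to the next.
; HackObject records the previous pawn and jump count, retargets the shared camera, possesses itself and calls a turret possess hook.
; BPHackingComponent picks the target each tick, hacks actors or terminals, and handles returns.
; Input toggles hacking mode, hacks, or backs out: short press to the previous pawn, long hold to the player.
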(event `/Game/blueprints/core/BPI_Interact.HackObject`
  (params (Controller :type "/Game/blueprints/core/BP_InGameController Object Reference") (lastActorPosses :type "Pawn Object Reference") (nbJump :type Integer) (camRef :type "/Game/blueprints/core/BP_PlayerCam Object Reference"))
  (set `self.distanceHack` nbJump)
  (set `self.Controller_0` Controller)
  (set `self.lastActorPosses` lastActorPosses)
  (bind _output_get (set `/Game/blueprints/core/BP_hackingComponent.RefCam` camRef (`self.BP_hackingComponent`)))
  (set `/Game/blueprints/core/BP_PlayerCam.focusWhichActor` self _output_get)
  (set `/Game/blueprints/core/BP_PlayerCam.offSetCam` (`self.offsetCamera`) _output_get)
  (`Controller.Possess` (`self.Controller_0`) self)
  (`self.possesTurret` (`self.Controller_0`)))

(event `/Game/blueprints/core/BPI_Interact.returnToLastActorPosses`
  (params (Controller :type "/Game/blueprints/core/BP_InGameController Object Reference"))
  (bind _refcam (`/Game/blueprints/core/BP_hackingComponent.RefCam` (`self.BP_hackingComponent`)))
  (set `/Game/blueprints/core/BP_hackingComponent.PawnInputs` "NewEnumerator0" (`self.BP_hackingComponent`))
  (`Controller.Possess` Controller self)
  (set `/Game/blueprints/core/BP_PlayerCam.focusWhichActor` self _refcam)
  (set `/Game/blueprints/core/BP_PlayerCam.offSetCam` (`self.offsetCamera`) _refcam))

(event `EnhancedInput|/Game/blueprints/core/Inputs/InputsActions/IA_Hack`
  (params (ActionValue :type Boolean) (ElapsedSeconds :type "Float (double-precision)") (TriggeredSeconds :type "Float (double-precision)") (InputAction :type "InputAction Object Reference" :default "/Game/blueprints/core/Inputs/InputsActions/IA_Hack.IA_Hack"))
  (:`Started`
    (bind _objecttohack (`self.ObjectToHack`)
      (:`then`
        (if (and (not (== (`GameplayStatics.GetObjectClass` (`self.ObjectToHack`)) "/Game/blueprints/core/BP_player.BP_player_C")) (not (== (`self.ObjectToHack`) (`self.lastActorPosses`))))
          (bind _asbp_actors_to_posses (cast `/Game/blueprints/BP_ActorsToPosses` _objecttohack)
            (:`then`
              (`/Game/blueprints/core/BP_hackingComponent.hackObject` (`self.BP_hackingComponent`) _asbp_actors_to_posses (`self.distanceHack`))
              (set `self.ObjectToHack` null))
            (:`CastFailed`
              (`/Game/blueprints/core/BP_hackingComponent.HackTerminal` (`self.BP_hackingComponent`) _objecttohack)))))
      (:`else`))))

(event `EnhancedInput|/Game/blueprints/core/Inputs/InputsActions/IA_switchMode`
  (params (ActionValue :type Boolean) (ElapsedSeconds :type "Float (double-precision)") (TriggeredSeconds :type "Float (double-precision)") (InputAction :type "InputAction Object Reference" :default "/Game/blueprints/core/Inputs/InputsActions/IA_switchMode.IA_switchMode"))
  (:`Started`
    (set `/Game/blueprints/core/BP_hackingComponent.PawnInputs` (select `/Game/blueprints/core/E_PlayerState` (`/Game/blueprints/core/BP_hackingComponent.PawnInputs` (`self.BP_hackingComponent`)) :`NewEnumerator0` (enumliteral `/Game/blueprints/core/E_PlayerState` "NewEnumerator3") :`NewEnumerator3` "NewEnumerator0") (`self.BP_hackingComponent`))))

(event `EnhancedInput|/Game/blueprints/core/Inputs/InputsActions/IA_backToLast`
  (params (ActionValue :type Boolean) (ElapsedSeconds :type "Float (double-precision)") (TriggeredSeconds :type "Float (double-precision)") (InputAction :type "InputAction Object Reference" :default "/Game/blueprints/core/Inputs/InputsActions/IA_backToLast.IA_backToLast"))
  (:`Triggered`
    (set `self.HoldToGetBackToPLayer` TriggeredSeconds))
  (:`Completed`
    (if (> (`self.HoldToGetBackToPLayer`) 1.0)
      (`/Game/blueprints/core/BP_hackingComponent.returnToPawnPlayer` (`self.BP_hackingComponent`))
      (`self.unPossessTurret`)
      (else
        (`/Game/blueprints/core/BP_hackingComponent.returnToLastActorPosses` (`self.BP_hackingComponent`) (`self.lastActorPosses`))
        (`self.unPossessTurret`)))))

(event `self.ReceiveTick`
  (params (DeltaSeconds :type "Float (single-precision)"))
  (bind _hit_result_hit_actor (`/Game/blueprints/core/BP_hackingComponent.setObjectToHack` (`self.BP_hackingComponent`)))
  (set `self.ObjectToHack` _hit_result_hit_actor))

(fn `UserConstructionScript`)