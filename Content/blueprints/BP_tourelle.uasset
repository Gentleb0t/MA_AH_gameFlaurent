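; Hackable turret that the player possesses to aim with the mouse in a side-view plane and fire.
; While possessed, Tick intersects the cursor ray with the actor's XZ plane and snaps RotationPoint to that pitch; the computed speed-scaled pitch is not applied.
; Holding IA_Hack in the matching hacking input state runs a looping fire timer until release.
; Shoot line-traces along the arrow and sends ShootedMessage to the hit actor.
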(event `self.ReceiveBeginPlay`
  (add `self.possesTurret` (delegate `possess`))
  (add `self.unPossessTurret` (delegate `unpossess`)))

(event `possess` :!signature `self.possesTurret`
  (params (Controller :type "/Game/blueprints/core/BP_customController Object Reference"))
  (set `self.as Controller` Controller)
  (set `self.isPossess` true))

(event `unpossess`
  (set `self.isPossess` false))

(event `EnhancedInput|/Game/blueprints/core/Inputs/InputsActions/IA_Hack`
  (params (ActionValue :type Boolean) (ElapsedSeconds :type "Float (double-precision)") (TriggeredSeconds :type "Float (double-precision)") (InputAction :type "InputAction Object Reference" :default "/Game/blueprints/core/Inputs/InputsActions/IA_Hack.IA_Hack"))
  (:`Triggered`
    (if (`|EnumEquality` (`/Game/blueprints/core/BP_hackingComponent.PawnInputs` (`self.BP_hackingComponent`)) "NewEnumerator0")
      (`/Engine/EditorBlueprintResources/StandardMacros.DoOnce` false :!label _label
        (:`Completed`
          (bind _returnvalue (`KismetSystemLibrary.K2_SetTimerDelegate` (`|CreateDelegate` :!event `Shoot`) (`self.ShootingRate`) true))
          (set `self.timerByEventShoot` _returnvalue)))))
  (:`Completed`
    (`KismetSystemLibrary.K2_ClearAndInvalidateTimerHandle` (`self.timerByEventShoot`))
    (goto _label :!via `Reset`)))

(event `self.ReceiveTick`
  (params (DeltaSeconds :type "Float (single-precision)"))
  (bind (_worldlocation _worlddirection) (`PlayerController.DeprojectMousePositionToWorld` (`self.as Controller`)))
  (if (`self.isPossess`)
    (bind _output_get (set `self.targetPitch` (`KismetMathLibrary.DegAtan2` (.z (- (`.Intersection` (`KismetMathLibrary.LinePlaneIntersection_OriginNormal` _worldlocation (* _worlddirection 1000000.0) (`self.K2_GetActorLocation`) (0.0 1.0 0.0))) (`SceneComponent.K2_GetComponentLocation` (`self.rotationPoint`)))) (.x (- (`.Intersection` (`KismetMathLibrary.LinePlaneIntersection_OriginNormal` _worldlocation (* _worlddirection 1000000.0) (`self.K2_GetActorLocation`) (0.0 1.0 0.0))) (`SceneComponent.K2_GetComponentLocation` (`self.rotationPoint`)))))))
    (bind _returnvalue (`KismetMathLibrary.NormalizeAxis` (- _output_get (`self.currentPitch`))))
    (set `self.Delta` _returnvalue)
    (set `self.currentPitch` (* DeltaSeconds _returnvalue (`self.speed`)))
    (`SceneComponent.K2_SetWorldRotation` (`self.rotationPoint`) (`KismetMathLibrary.MakeRotator` 0.0 (`self.targetPitch`)) false false)))

(fn `Shoot`
  (locals (rangeShoot :type "Float (double-precision)" :default 1500.0))
  (bind _returnvalue (`SceneComponent.K2_GetComponentLocation` (`self.rotationPoint`)))
  (bind _outhit (`KismetSystemLibrary.LineTraceSingle` :`Start` _returnvalue :`End` (+ _returnvalue (* (`SceneComponent.GetForwardVector` (`self.Arrow`)) (`local.rangeShoot`))) :`TraceChannel` "TraceTypeQuery1" :`DrawDebugType` "ForDuration"))
  (message `/Game/blueprints/core/BPI_Combat.shooted` (`.HitActor` (`GameplayStatics.BreakHitResult` _outhit))))

(fn `UserConstructionScript`
  (`parent.UserConstructionScript`))