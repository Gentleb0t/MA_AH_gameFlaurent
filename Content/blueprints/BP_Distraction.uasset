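; BP_Distraction is a distraction source that alerts nearby actors to its location.
; StartDistraction runs a zero-length multi-sphere trace on the Visibility channel, centered on the actor with radius RangeDistraction.
; Each hit actor receives a DistractionMessage carrying the source's location, leaving the response to the receiver.
; The trace leaves persistent debug drawing enabled.
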(event `self.ReceiveBeginPlay`
  (`parent.ReceiveBeginPlay`))

(event `StartDistraction`
  (`self.StartDistractionToActors`))

(fn `StartDistractionToActors`
  (bind _returnvalue (`self.K2_GetActorLocation`))
  (bind _outhits (`KismetSystemLibrary.SphereTraceMulti` :`Start` _returnvalue :`End` _returnvalue :`Radius` (`self.RangeDistraction`) :`TraceChannel` "TraceTypeQuery1" :`DrawDebugType` "Persistent"))
  (for _array_element _outhits
    (message `/Game/blueprints/core/BPI_Common.distraction` (`.HitActor` (`GameplayStatics.BreakHitResult` _array_element)) (`self.K2_GetActorLocation`))))

(fn `UserConstructionScript`
  (`parent.UserConstructionScript`))