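; BP_Door is a door actor that slides downward to open when it is hacked.
; On BeginPlay it binds to its BPReceiver's Hacked event, stores its start location and scales the OpenDoor timeline's play rate by ElevatorTrajectoryTime.
; When hacked, the timeline lerps the actor from that origin to a fixed offset below it, without sweep.
; The file contains no closing logic.
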(event `self.ReceiveBeginPlay`
  (`parent.ReceiveBeginPlay`)
  (add `/Game/blueprints/BP_Interactions.hacked` (`self.BP_receiver`) (delegate `OpenDoorAnim`))
  (set `self.origineLoc` (`self.K2_GetActorLocation`))
  (`TimelineComponent.SetPlayRate` (`self.openDoor`) (/ 1.0 (`self.Elevator Trajectory Time`))))

(event `OpenDoorAnim`
  (bind _origineloc (`self.origineLoc`))
  (bind (_direction _newtrack_1) (`Timeline|openDoor`)
    (:`Update`
      (`self.K2_SetActorLocation` (`KismetMathLibrary.VLerp` _origineloc (- _origineloc (0.0 0.0 500.0)) _newtrack_1)))))

(fn `UserConstructionScript`
  (`parent.UserConstructionScript`))