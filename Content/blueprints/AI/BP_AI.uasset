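; BP_AI is a patrolling AI that detects the player by perception and is destroyed when shot.
; BeginPlay seeds the Blackboard with the spawn location and first path point, and sight updates set or clear the player reference there.
; CheckNextPoint advances through paired location and wait-time arrays via NextPoint.
; At the path's end it resets the index and targets the actor's current location, not the stored origin.
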(event `self.ReceiveBeginPlay`
  ; initialisation du blackboard
  (set `self.blackboardRef` (`AIBlueprintHelperLibrary.GetBlackboard` null))
  (`self.initBlackBoard`))

(event `self.Sight.OnTargetPerceptionInfoUpdated`
  (params (UpdateInfo :type "ActorPerceptionUpdateInfo Structure (by ref)"))
  ; gère si l'IA voit ou non le player et actualise le BlackBoard
  (cast `/Game/blueprints/core/BP_player` UpdateInfo_Target)
  (if (`.bSuccessfullySensed` (break `AIStimulus` (`.Stimulus` (break `ActorPerceptionUpdateInfo` UpdateInfo))))
    (`BlackboardComponent.SetValueAsObject` (`self.blackboardRef`) "playerRef" UpdateInfo_Target)
    (else
      (`BlackboardComponent.ClearValue` (`self.blackboardRef`) "playerRef"))))

(event `/Game/blueprints/core/BPI_Combat.shooted`
  (`self.K2_DestroyActor`))

(fn `CheckNextPoint`
  ; si pendant la ronde il arrive a la fin recommance la ronde en retournant a son point de départ
  (if (== (`self.indexWichPointToGo`) (- (`KismetArrayLibrary.Array_Length` (`self.Path`)) 1))
    (set `self.indexWichPointToGo` 0)
    (`self.NextPoint` (`self.K2_GetActorLocation`) (`self.waitTimeStartPoint`))
    (else
      (bind _result (`/Engine/EditorBlueprintResources/StandardMacros.IncrementInt` (`self.indexWichPointToGo`))
        (:`  `
          (`self.NextPoint` (`|GetArrayItem` (`self.Path`) _result) (`|GetArrayItem` (`self.WaitTillNextPathPoint`) _result)))))))

(fn `initBlackBoard`
  (bind _path (`self.Path`))
  (`|ExecutionSequence`
    (:`then_0`
      ; si au moins 1 points est donnée dans le chemin alors il va executer la boucle de mouvement
      (if (`KismetArrayLibrary.Array_IsNotEmpty` _path)
        (`self.NextPoint` (`|GetArrayItem` _path) (`|GetArrayItem` (`self.WaitTillNextPathPoint`)))))
    (:`then_1`
      ; Comment
      (`BlackboardComponent.SetValueAsVector` (`self.blackboardRef`) "OriginePoint" (`self.K2_GetActorLocation`)))))

(fn `NextPoint`
  (params (VectorValue :type "Vector Structure") (FloatValue :type "Float (double-precision)"))
  ; prend un poind dans le monde et un temp d'attente et le set dans le blackboard
  (`BlackboardComponent.SetValueAsVector` (`self.blackboardRef`) "locationToFollow" VectorValue)
  (`BlackboardComponent.SetValueAsFloat` (`self.blackboardRef`) "waitTime" FloatValue))

(fn `UserConstructionScript`)